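; Level 1 alien enemy that wanders the navmesh, attacks the player on sight, and drops an item when killed.
; Tick issues random AIMoveTo calls, gated by the DoitAvancer and EnMouvement flags.
; PawnSensing triggers a chase that takes one Vie from the player on arrival, and also spawns a Laser_Alien from Arrow3.
; A FirstPersonProjectile hit spawns BP_Item_lvl1, increments the player's AlienMorts and destroys the alien.
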(event `self.ReceiveTick`
  (params (DeltaSeconds :type "Float (single-precision)"))
  ;[1 1 1] Mouvement Aléatoires
  (`|ExecutionSequence`
    (:`then_1`
      (if (== (`self.Doit_Avancer`) false)
        (if (== (`self.En_mouvement`) false)
          (set `self.En_mouvement` true)
          (`|AIMoveTo` self (`NavigationSystem.K2_GetRandomLocationInNavigableRadius` (`self.K2_GetActorLocation`) 50000.0)
            (:`OnSuccess`
              _)
            (:`OnFail`
              _))
          (set `self.En_mouvement` false))))))

(event `self.PawnSensing.OnSeePawn`
  (params (Pawn :type "Pawn Object Reference"))
  (bind _arrow3 (`self.Arrow3`))
  ;[1 1 1] IA
  (set `self.Doit_Avancer` true)
  (set `self.En_mouvement` true)
  (bind _asfirst_person_character (cast `/Game/FirstPersonBP/Blueprints/FirstPersonCharacter` Pawn))
  (`|ExecutionSequence`
    (:`then_0`
      (`|AIMoveTo` self (`self.K2_GetActorLocation` (`GameplayStatics.GetPlayerCharacter` 0)) _asfirst_person_character
        (:`OnSuccess`
          (set `self.Doit_Avancer` false)
          (set `self.En_mouvement` false)
          (bind _asfirst_person_character_2 (cast `/Game/FirstPersonBP/Blueprints/FirstPersonCharacter` (`GameplayStatics.GetPlayerCharacter` 0)))
          (set `/Game/FirstPersonBP/Blueprints/FirstPersonCharacter.Vie` (- (`/Game/FirstPersonBP/Blueprints/FirstPersonCharacter.Vie` _asfirst_person_character_2) 1) _asfirst_person_character_2))))
    (:`then_1`
      (bind _output_get (set `self.NewVar_0` (`KismetMathLibrary.MakeTransform` (`SceneComponent.K2_GetComponentLocation` _arrow3) (`SceneComponent.K2_GetComponentRotation` _arrow3))))
      (`|SpawnActorFromClass` "/Game/FirstPersonBP/Blueprints/Laser_Alien.Laser_Alien_C" _output_get "AlwaysSpawn" "OverrideRootScale") ; Spawn projectile
    )))

(event `self.Collision.OnComponentHit`
  (params (HitComponent :type "PrimitiveComponent Object Reference") (OtherActor :type "Actor Object Reference") (OtherComp :type "PrimitiveComponent Object Reference") (NormalImpulse :type "Vector Structure") (Hit :type "HitResult Structure (by ref)"))
  (bind (_returnvalue_location _returnvalue_rotation) (`KismetMathLibrary.BreakTransform` (`SceneComponent.K2_GetComponentToWorld` (`self.Arrow1`))))
  ;[1 1 1] Mort
  (`KismetSystemLibrary.PrintString` "Touché")
  (cast `/Game/FirstPersonBP/Blueprints/FirstPersonProjectile` OtherActor)
  (`|SpawnActorFromClass` "/Game/Blueprint/Item/BP_Item_lvl1.BP_Item_lvl1_C" (`KismetMathLibrary.MakeTransform` _returnvalue_location _returnvalue_rotation (0.75 0.75 0.75)) "Undefined" "OverrideRootScale")
  (bind _asfirst_person_character (cast `/Game/FirstPersonBP/Blueprints/FirstPersonCharacter` (`GameplayStatics.GetPlayerCharacter` 0)))
  (set `/Game/FirstPersonBP/Blueprints/FirstPersonCharacter.Alien_morts` (+ (`/Game/FirstPersonBP/Blueprints/FirstPersonCharacter.Alien_morts` _asfirst_person_character) 1) _asfirst_person_character)
  (`self.K2_DestroyActor`))

(event `self.ReceiveBeginPlay`
  ;[1 1 1] Animation Marche
  (`SkeletalMeshComponent.PlayAnimation` (`self.Mesh`) "/Game/Anim/Alien_LVL1_Avance.Alien_LVL1_Avance" false))

(fn `UserConstructionScript`)