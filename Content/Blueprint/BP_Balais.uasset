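; BP_Balais is a broom pickup that highlights when seen and can be collected by the first-person character.
; BalaisVu enables custom depth rendering on the broom and sets the VU flag, while Tick clears both every frame, so the highlight lasts only while BalaisVu keeps being called.
; Ramasser notifies FirstPersonCharacter through BalaisRammassé, then destroys the actor.
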(event `Ramasser`
  ;[1 1 1] Rammasser
  (bind _asfirst_person_character (cast `/Game/FirstPersonBP/Blueprints/FirstPersonCharacter` (`GameplayStatics.GetPlayerCharacter` 0)))
  (`/Game/FirstPersonBP/Blueprints/FirstPersonCharacter.BalaisRammassé` _asfirst_person_character)
  (`self.K2_DestroyActor`))

(event `BalaisVu`
  ;[1 1 1] Balais vu
  (`PrimitiveComponent.SetRenderCustomDepth` (`self.Balais`) true)
  (set `self.VU` true))

(event `self.ReceiveTick`
  (params (DeltaSeconds :type "Float (single-precision)"))
  (`|ExecutionSequence`
    (:`then_0`
      (`PrimitiveComponent.SetRenderCustomDepth` (`self.Balais`) false)
      (set `self.VU` false))))

(fn `UserConstructionScript`)