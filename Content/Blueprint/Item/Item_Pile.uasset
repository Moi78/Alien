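; Pickup item for a "Pile" that the first-person player can highlight and collect into the inventory.
; The Vu event turns on custom depth and a seen flag, which Tick clears so they hold only while Vu keeps firing.
; After a delayed input enable on BeginPlay, pressing E while seen sets the character's CaseInventaire, updates the Status widget's inventory icon and destroys the actor.
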(event `self.ReceiveBeginPlay`
  (`KismetSystemLibrary.Delay` 11.3)
  (`self.EnableInput` (`GameplayStatics.GetPlayerController` 0)))

(event `Key|E` :consume false
  (params (Key :type "Key Structure" :default "AnyKey"))
  (:`Pressed`
    (if (and (`self.EstVu`) (!= (`self.EstPris`) true))
      (bind _asfirst_person_character (cast `/Game/FirstPersonBP/Blueprints/FirstPersonCharacter` (`GameplayStatics.GetPlayerCharacter` 0)))
      (set `/Game/FirstPersonBP/Blueprints/FirstPersonCharacter.CaseInventaire` "Item_Pile_C" _asfirst_person_character)
      (set `self.EstPris` true)
      (bind _foundwidgets (`WidgetBlueprintLibrary.GetAllWidgetsOfClass` "/Game/HUDS/Status/Status.Status_C"))
      (`/Game/HUDS/Status/Status.Set img inventaire` (`|GetArrayItem` _foundwidgets) "/Game/HUDS/Status/Inventaire/Icônes/PileIco.PileIco")
      (`self.K2_DestroyActor`))))

(event `Vu`
  (`PrimitiveComponent.SetRenderCustomDepth` (`self.Pile_Model`) true)
  (set `self.EstVu` true))

(event `self.ReceiveTick`
  (params (DeltaSeconds :type "Float (single-precision)"))
  (`PrimitiveComponent.SetRenderCustomDepth` (`self.Pile_Model`) false)
  (set `self.EstVu` false))

(fn `UserConstructionScript`)