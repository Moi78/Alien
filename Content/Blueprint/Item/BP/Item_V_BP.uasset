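; Item_V_BP is a collectible pickup that spins its static mesh slightly every tick.
; When the FirstPersonCharacter overlaps its box, it increments that character's NbItemV count and prints it.
; It then adds points to ScoreTotal on player 0's character, fetched separately from the overlapping actor, and destroys itself.
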(event `self.ReceiveTick`
  (params (DeltaSeconds :type "Float (single-precision)"))
  (`SceneComponent.K2_AddLocalRotation` (`self.StaticMesh`) (struct :`Yaw` 0.5) false false))

(event `self.Box.OnComponentBeginOverlap`
  (params (OverlappedComponent :type "PrimitiveComponent Object Reference") (OtherActor :type "Actor Object Reference") (OtherComp :type "PrimitiveComponent Object Reference") (OtherBodyIndex :type Integer) (bFromSweep :type Boolean) (SweepResult :type "HitResult Structure (by ref)"))
  (bind _asfirst_person_character (cast `/Game/FirstPersonBP/Blueprints/FirstPersonCharacter` OtherActor))
  (bind _output_get (set `/Game/FirstPersonBP/Blueprints/FirstPersonCharacter.Nb_Item_V` (+ (`/Game/FirstPersonBP/Blueprints/FirstPersonCharacter.Nb_Item_V` _asfirst_person_character) 1) _asfirst_person_character))
  (`KismetSystemLibrary.PrintString` (`KismetStringLibrary.Conv_IntToString` _output_get))
  (bind _asfirst_person_character_2 (cast `/Game/FirstPersonBP/Blueprints/FirstPersonCharacter` (`GameplayStatics.GetPlayerCharacter` 0)))
  (set `/Game/FirstPersonBP/Blueprints/FirstPersonCharacter.score_total` (+ (`/Game/FirstPersonBP/Blueprints/FirstPersonCharacter.score_total` _asfirst_person_character_2) 10) _asfirst_person_character_2)
  (`self.K2_DestroyActor`))

(fn `UserConstructionScript`)