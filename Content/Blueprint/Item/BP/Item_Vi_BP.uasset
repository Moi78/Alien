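; Item_Vi_BP is a spinning "Vi" item that counts toward the player character's item tally.
; Tick rotates the static mesh by a fixed step each frame, independent of delta time.
; A box overlap by FirstPersonCharacter increments that character's NbItemVi but leaves the item in place.
; Disconnected nodes that would print, add to ScoreTotal and destroy the actor never run.
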(event `self.ReceiveTick`
  (params (DeltaSeconds :type "Float (single-precision)"))
  (`SceneComponent.K2_AddLocalRotation` (`self.StaticMesh`) (struct :`Yaw` 0.5) false false))

(event `self.Box.OnComponentBeginOverlap`
  (params (OverlappedComponent :type "PrimitiveComponent Object Reference") (OtherActor :type "Actor Object Reference") (OtherComp :type "PrimitiveComponent Object Reference") (OtherBodyIndex :type Integer) (bFromSweep :type Boolean) (SweepResult :type "HitResult Structure (by ref)"))
  (bind _asfirst_person_character (cast `/Game/FirstPersonBP/Blueprints/FirstPersonCharacter` OtherActor))
  (set `/Game/FirstPersonBP/Blueprints/FirstPersonCharacter.Nb Item Vi` (+ (`/Game/FirstPersonBP/Blueprints/FirstPersonCharacter.Nb Item Vi` _asfirst_person_character) 1) _asfirst_person_character))

(fn `UserConstructionScript`)