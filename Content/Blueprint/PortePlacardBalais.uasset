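; Broom closet door that opens when the player character enters the button's trigger box.
; The overlap recolors the button through its Couleur material parameter and plays the Ouverture timeline from the start.
; Each timeline update adds the track value to the door's local offset, so movement accumulates per tick.
; EstOuvert gates the trigger but is never set in this graph, so re-entering can replay the opening.
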(event `OuvertureP`
  ;[1 1 1] Anim Ouverture
  (bind (_direction _newtrack_0) (`Timeline|Ouverture` :!via `PlayFromStart`)
    (:`Update`
      (`SceneComponent.K2_AddLocalOffset` (`self.Porte`) _newtrack_0 false false))))

(event `self.Box.OnComponentBeginOverlap`
  (params (OverlappedComponent :type "PrimitiveComponent Object Reference") (OtherActor :type "Actor Object Reference") (OtherComp :type "PrimitiveComponent Object Reference") (OtherBodyIndex :type Integer) (bFromSweep :type Boolean) (SweepResult :type "HitResult Structure (by ref)"))
  ;[1 1 1] Bouton
  (if (and (== OtherActor (`GameplayStatics.GetPlayerCharacter` 0)) (== (`self.EstOuvert`) false))
    (`MeshComponent.SetVectorParameterValueOnMaterials` (`self.bouton`) "Couleur" (0.0 0.5 1.0))
    (`self.OuvertureP`)))

(fn `UserConstructionScript`)