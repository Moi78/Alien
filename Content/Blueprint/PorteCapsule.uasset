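; Capsule door Blueprint that plays an animated unlock-and-open sequence when its Ouvrir event is called.
; Two timelines start together, Verrou_Haut moving locks 1 and 2 and Verrou_Bas moving locks 3 and 4.
; When Verrou_Bas finishes, PortePrincipaleOuverture moves the main door panel.
; Timeline values are added as local offsets on every update without sweep, so travel accumulates per tick rather than following absolute positions.
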(event `Ouvrir`
  (`|ExecutionSequence`
    (:`then_0`
      (bind (_direction _verrou_haut) (`Timeline|Verrou_Haut`)
        (:`Update`
          (`|ExecutionSequence`
            (:`then_0`
              (`SceneComponent.K2_AddLocalOffset` (`self.PorteCapsule_Verrou1`) _verrou_haut false false))
            (:`then_1`
              (`SceneComponent.K2_AddLocalOffset` (`self.PorteCapsule_Verrou2`) _verrou_haut false false))))))
    (:`then_1`
      (bind (_direction_2 _verrou_bas) (`Timeline|Verrou_Bas`)
        (:`Update`
          (`|ExecutionSequence`
            (:`then_0`
              (`SceneComponent.K2_AddLocalOffset` (`self.PorteCapsule_Verrou3`) _verrou_bas false false))
            (:`then_1`
              (`SceneComponent.K2_AddLocalOffset` (`self.PorteCapsule_Verrou4`) _verrou_bas false false))))
        (:`Finished`
          (bind (_direction_3 _newtrack_0) (`Timeline|PortePrincipaleOuverture`)
            (:`Update`
              (`SceneComponent.K2_AddLocalOffset` (`self.PorteCapsule_Porte`) _newtrack_0 false false))))))))

(fn `UserConstructionScript`)