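; Door Blueprint with a trigger button that opens a pair of door panels once when the first-person character steps into its box.
; The overlap recolours the Bouton material through its Couleur parameter, calls Ouverture, then destroys the trigger.
; Ouverture plays the Porte timeline, whose two tracks feed AddLocalOffset on PORTED and PORTEG each update, so the offsets accumulate rather than setting absolute positions.
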(event `Ouverture`
  ;[1 1 1] Anim Porte Entrée
  (bind (_direction _ported _porteg) (`Timeline|Porte`)
    (:`Update`
      (`|ExecutionSequence`
        (:`then_0`
          (`SceneComponent.K2_AddLocalOffset` (`self.PORTE_D`) _ported false false))
        (:`then_1`
          (`SceneComponent.K2_AddLocalOffset` (`self.PORTE_G`) _porteg false false))))))

(event `self.Box.OnComponentBeginOverlap`
  (params (OverlappedComponent :type "PrimitiveComponent Object Reference") (OtherActor :type "Actor Object Reference") (OtherComp :type "PrimitiveComponent Object Reference") (OtherBodyIndex :type Integer) (bFromSweep :type Boolean) (SweepResult :type "HitResult Structure (by ref)"))
  ;[1 1 1] Bouton
  (cast `/Game/FirstPersonBP/Blueprints/FirstPersonCharacter` OtherActor)
  (`MeshComponent.SetVectorParameterValueOnMaterials` (`self.Bouton`) "Couleur" (0.0 0.5 1.0))
  (`self.Ouverture`)
  (`ActorComponent.K2_DestroyComponent` OverlappedComponent))

(fn `UserConstructionScript`)