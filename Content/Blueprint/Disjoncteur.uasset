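; Circuit breaker (Disjoncteur) that powers up with a battery and opens the capsule door (PorteCapsule).
; Vu sets a looked-at flag and custom-depth highlight, which Tick clears every frame; input is enabled after a startup delay.
; E shows the battery model, empties the player's inventory slot and HUD image, greens the light and calls Ouvrir on the door.
; The looked-at and held-battery check gates nothing as wired.
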(event `self.ReceiveBeginPlay`
  (`KismetSystemLibrary.Delay` 11.3)
  (`self.EnableInput` (`GameplayStatics.GetPlayerController` 0)))

(event `Key|E` :consume false
  (params (Key :type "Key Structure" :default "AnyKey"))
  (:`Pressed`
    (bind _asfirst_person_character (cast `/Game/FirstPersonBP/Blueprints/FirstPersonCharacter` (`GameplayStatics.GetPlayerCharacter` 0)))
    (if (and (`self.EstVu`) (== (`/Game/FirstPersonBP/Blueprints/FirstPersonCharacter.CaseInventaire` _asfirst_person_character) "/Game/Blueprint/Item/Item_Pile.Item_Pile_C"))
      _
      (else
        _))
    (`SceneComponent.SetVisibility` (`self.Pile_Model`) true false)
    (bind _asfirst_person_character_2 (cast `/Game/FirstPersonBP/Blueprints/FirstPersonCharacter` (`GameplayStatics.GetPlayerCharacter` 0)))
    (set `/Game/FirstPersonBP/Blueprints/FirstPersonCharacter.CaseInventaire` null _asfirst_person_character_2)
    (bind _foundwidgets (`WidgetBlueprintLibrary.GetAllWidgetsOfClass` "/Game/HUDS/Status/Status.Status_C"))
    (`/Game/HUDS/Status/Status.Set img inventaire` (`|GetArrayItem` _foundwidgets) "/Engine/EngineResources/WhiteSquareTexture.WhiteSquareTexture")
    (set `self.EstActivé` true)
    (`LightComponent.SetLightColor` (`self.PointLight`) (struct :`R` 0.057249 :`G` 1.0 :`A` 1.0) true)
    (bind _outactors (`GameplayStatics.GetAllActorsOfClass` "/Game/Blueprint/PorteCapsule.PorteCapsule_C"))
    (`/Game/Blueprint/PorteCapsule.Ouvrir` (`|GetArrayItem` _outactors))))

(event `Vu`
  (`PrimitiveComponent.SetRenderCustomDepth` (`self.Disjoncteur`) true)
  (set `self.EstVu` true))

(event `self.ReceiveTick`
  (params (DeltaSeconds :type "Float (single-precision)"))
  (`PrimitiveComponent.SetRenderCustomDepth` (`self.Disjoncteur`) false)
  (set `self.EstVu` false))

(fn `UserConstructionScript`)